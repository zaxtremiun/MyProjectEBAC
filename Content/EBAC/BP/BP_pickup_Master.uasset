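; BP_pickup_Master is a master pickup actor whose Item data is loaded from a data table row in the construction script.
; Overlapping its collision registers it as the player's last interact object and look-at target, and sets CantInteract, which despite its name enables interaction.
; Leaving clears CantInteract and the look-at flag.
; The interact event, when enabled, calls the empty item-picked-up event, likely a child hook, then destroys the actor.
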(event `self.colision.OnComponentEndOverlap`
  (params (OverlappedComponent :type "PrimitiveComponent Object Reference") (OtherActor :type "Actor Object Reference") (OtherComp :type "PrimitiveComponent Object Reference") (OtherBodyIndex :type Integer))
  ; Quando sair da area de colisao cantINteract é falso
  (bind _asbp_third_person_character_player (cast `/Game/ThirdPerson/Blueprints/BP_ThirdPersonCharacter_Player` OtherActor))
  (set `self.CantInteract?` false)
  (set `/Game/ThirdPerson/Blueprints/BP_ThirdPersonCharacter_Player.loockatt?_0` false _asbp_third_person_character_player)
  (`KismetSystemLibrary.PrintString` "lookoff"))

(event `self.ALGO.OnComponentEndOverlap`
  (params (OverlappedComponent :type "PrimitiveComponent Object Reference") (OtherActor :type "Actor Object Reference") (OtherComp :type "PrimitiveComponent Object Reference") (OtherBodyIndex :type Integer)))

(event `self.colision.OnComponentBeginOverlap`
  (params (OverlappedComponent :type "PrimitiveComponent Object Reference") (OtherActor :type "Actor Object Reference") (OtherComp :type "PrimitiveComponent Object Reference") (OtherBodyIndex :type Integer) (bFromSweep :type Boolean) (SweepResult :type "HitResult Structure (by ref)"))
  ; quando entra em colisao cant INteract é true
  (bind _asbp_third_person_character_player (cast `/Game/ThirdPerson/Blueprints/BP_ThirdPersonCharacter_Player` OtherActor))
  (set `/Game/ThirdPerson/Blueprints/BP_ThirdPersonCharacter_Player.LAstINteractOBJ_0` self _asbp_third_person_character_player)
  (set `self.CantInteract?` true)
  ; set lookPosition
  (set `/Game/ThirdPerson/Blueprints/BP_ThirdPersonCharacter_Player.loockatt?_0` true _asbp_third_person_character_player)
  (set `/Game/ThirdPerson/Blueprints/BP_ThirdPersonCharacter_Player.lockattactor_0` self _asbp_third_person_character_player))

(event `DEB_Item_Que_Pegou`)

(event `/Game/EBAC/BP/BPI_interact.INteractive`
  (if (`self.CantInteract?`)
    (`KismetSystemLibrary.Delay` 0.0)
    (`self.DEB_item_que_pegou`)
    (`self.K2_DestroyActor`)))

(fn `UserConstructionScript`
  (bind (_datatable _rowname) (break `DataTableRowHandle` (`self.Data Table Row Handle`)))
  (bind _returnvalue (`|GetDataTableRow` _datatable _rowname)
    (:`then`
      (bind _output_get (set `self.item` _returnvalue)))))