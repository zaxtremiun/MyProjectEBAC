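; BP_enemy_bat is a bat enemy whose logic here is a single attack event that hurts the player.
; When atk fires, it checks whether AtkBox overlaps the player character, applies fixed damage and writes the resulting health fraction straight to the player's HUD progress bar.
; Nothing in this graph triggers atk, as BeginPlay, overlap and Tick are unused.
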(event `atk`
  (bind _returnvalue (`GameplayStatics.GetPlayerCharacter` 0))
  (if (`PrimitiveComponent.IsOverlappingActor` (`self.AtkBox`) _returnvalue)
    (bind _asbp_third_person_character_player (cast `/Game/ThirdPerson/Blueprints/BP_ThirdPersonCharacter_Player` _returnvalue))
    (`/Game/ThirdPerson/Blueprints/BP_ThirdPersonCharacter_Player.dammage` _asbp_third_person_character_player 10.0)
    (`ProgressBar.SetPercent` (`/Game/EBAC/HUD/HUD_Player.PROGRSS_HEALTH` (`/Game/ThirdPerson/Blueprints/BP_ThirdPersonCharacter_Player.HUD_Health_0` _asbp_third_person_character_player)) (/ (`.health_7_F21391B646F991367FAD1493A83BC0DC` (break `/Game/ThirdPerson/Blueprints/S_stats` (`/Game/ThirdPerson/Blueprints/BP_Master_Character.stats` _asbp_third_person_character_player))) 100.0))))

(fn `UserConstructionScript`)