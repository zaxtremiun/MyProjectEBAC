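; AI controller that starts the Enemy_BH behavior tree when play begins.
; All other logic is unconnected and never runs.
; Those leftovers include a blackboard write of the player's location and a chase loop that retries MoveToActor after a delay and calls Atk on BP_enemy_bat when already at the player.
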(event `self.ReceiveBeginPlay`
  (`self.RunBehaviorTree` "/Game/EBAC/BP/IA/Enemy_BH.Enemy_BH"))

(fn `UserConstructionScript`)