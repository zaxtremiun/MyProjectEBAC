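; BP_SpawMagic handles player spellcasting through an enchantment mode and rune inputs that choose which magic ball to spawn.
; A toggle enables rune input, storing the element and class in one slot; only air fills an empty slot, while fire, rock and water require it filled.
; Activating spawns that class at an offset and ends enchantment without clearing the slot.
; Right mouse separately spawns a waterball, spending mana and updating the HUD.
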(event `EnhancedInput|/Game/EBAC/BP/magics/IA_Rune_air`
  (params (ActionValue :type Boolean) (ElapsedSeconds :type "Float (double-precision)") (TriggeredSeconds :type "Float (double-precision)") (InputAction :type "InputAction Object Reference" :default "/Game/EBAC/BP/magics/IA_Rune_air.IA_Rune_air"))
  (:`Triggered`
    (if (`self.enchantment_on?`)
      (if (not (`self.slot1used?`))
        (set `self.slot1used?` true)
        (set `self.slot1V` 1)
        (set `self.magictype` "/Game/EBAC/BP/BP_Airball.BP_Airball_C")
        (`KismetSystemLibrary.PrintString` "rune air")))))

(event `EnhancedInput|/Game/EBAC/BP/magics/IA_Rune_fire`
  (params (ActionValue :type Boolean) (ElapsedSeconds :type "Float (double-precision)") (TriggeredSeconds :type "Float (double-precision)") (InputAction :type "InputAction Object Reference" :default "/Game/EBAC/BP/magics/IA_Rune_fire.IA_Rune_fire"))
  (:`Triggered`
    (if (`self.enchantment_on?`)
      (if (`self.slot1used?`)
        (set `self.slot1used?` true)
        (set `self.slot1V` 2)
        (set `self.magictype` "/Game/EBAC/BP/BP_fireball.BP_fireball_C")
        (`KismetSystemLibrary.PrintString` "rune fire")))))

(event `EnhancedInput|/Game/EBAC/BP/magics/IA_Rune_rock`
  (params (ActionValue :type Boolean) (ElapsedSeconds :type "Float (double-precision)") (TriggeredSeconds :type "Float (double-precision)") (InputAction :type "InputAction Object Reference" :default "/Game/EBAC/BP/magics/IA_Rune_rock.IA_Rune_rock"))
  (:`Triggered`
    (if (`self.enchantment_on?`)
      (if (`self.slot1used?`)
        (set `self.slot1used?` true)
        (set `self.slot1V` 3)
        (set `self.magictype` "/Game/EBAC/BP/BP_rockball.BP_rockball_C")
        (`KismetSystemLibrary.PrintString` "rune rock")))))

(event `EnhancedInput|/Game/EBAC/BP/magics/IA_Rune_water`
  (params (ActionValue :type Boolean) (ElapsedSeconds :type "Float (double-precision)") (TriggeredSeconds :type "Float (double-precision)") (InputAction :type "InputAction Object Reference" :default "/Game/EBAC/BP/magics/IA_Rune_water.IA_Rune_water"))
  (:`Triggered`
    (if (`self.enchantment_on?`)
      (if (`self.slot1used?`)
        (set `self.slot1used?` true)
        (set `self.slot1V` 4)
        (set `self.magictype` "/Game/EBAC/BP/BP_Waterballball.BP_Waterballball_C")
        (`KismetSystemLibrary.PrintString` "rune water")))))

(event `EnhancedInput|/Game/EBAC/BP/magics/IA_activeSpell`
  (params (ActionValue :type Boolean) (ElapsedSeconds :type "Float (double-precision)") (TriggeredSeconds :type "Float (double-precision)") (InputAction :type "InputAction Object Reference" :default "/Game/EBAC/BP/magics/IA_activeSpell.IA_activeSpell"))
  (bind (_returnvalue_location _returnvalue_rotation) (`KismetMathLibrary.BreakTransform` (`self.GetTransform`)))
  (:`Triggered`
    (if (`self.enchantment_on?`)
      (if (`self.slot1used?`)
        (`|SpawnActorFromClass` (`self.magictype`) (`KismetMathLibrary.MakeTransform` (+ _returnvalue_location (40.0 0.0 0.0)) _returnvalue_rotation (0.5 0.5 0.5)) "AlwaysSpawn" "MultiplyWithRoot" null null)
        (set `self.enchantment_on?` false)
        (else
          (`KismetSystemLibrary.PrintString` "Hello")
          (set `self.enchantment_on?` false))))))

(event `EnhancedInput|/Game/EBAC/BP/magics/enchantment_Mode`
  (params (ActionValue :type Boolean) (ElapsedSeconds :type "Float (double-precision)") (TriggeredSeconds :type "Float (double-precision)") (InputAction :type "InputAction Object Reference" :default "/Game/EBAC/BP/magics/enchantment_Mode.enchantment_Mode"))
  (:`Triggered`
    (`/Engine/EditorBlueprintResources/StandardMacros.FlipFlop`
      (:`A`
        (`KismetSystemLibrary.PrintString` "enchantment on")
        (set `self.enchantment_on?` true))
      (:`B`
        (`KismetSystemLibrary.PrintString` "enchantment off")
        (set `self.enchantment_on?` false)))))

(event `Key|RightMouseButton`
  (params (Key :type "Key Structure"))
  (bind (_returnvalue_location _returnvalue_rotation) (`KismetMathLibrary.BreakTransform` (`self.GetTransform`)))
  ; Spaw waterball
  (:`Pressed`
    (if (>= (`self.ManaPlayer`) 20.0)
      (`KismetSystemLibrary.PrintString` "waterball")
      (bind _output_get (set `self.ManaPlayer` (- (`self.ManaPlayer`) 20.0)))
      (`ProgressBar.SetPercent` (`/Game/EBAC/HUD/HUD_Player.PROGRESS_MANA` (`self.HUD_Health`)) (/ _output_get 100.0))
      (`|SpawnActorFromClass` "/Game/EBAC/BP/BP_Waterballball.BP_Waterballball_C" (`KismetMathLibrary.MakeTransform` (+ _returnvalue_location (30.0 0.0 0.0)) _returnvalue_rotation (0.5 0.5 0.5)) "AlwaysSpawn" "MultiplyWithRoot" null null)
      (else
        (`KismetSystemLibrary.PrintString` "insufficient mana ")))))

(fn `UserConstructionScript`)